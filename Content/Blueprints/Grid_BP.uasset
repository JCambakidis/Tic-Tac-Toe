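; Tic-tac-toe style board actor that spawns the boxes and detects wins or a full board.
; The construction script lays out centered rows and columns of indexed Box_BP child actors, each referencing the grid.
; CheckEnd tests lines through the center and edge-middle boxes via CheckSides, using hard-coded 3x3 index offsets, to set the winner.
; A Gate closed by any unclaimed box flags game end when the board is full.
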(event `self.ReceiveTick`
  (params (DeltaSeconds :type "Float (single-precision)")))

(event `Check End`
  (`|ExecutionSequence`
    (:`then_0`
      (for _array_element (`self.Boxs`) :!label _label
        (if (!= (`/Game/Blueprints/Box_BP.Clicked_Player` _array_element) -1)
          (bind _index (`/Game/Blueprints/Box_BP.Index` _array_element))
          (if (== _index 4)
            (for _index_2 (range 1 (+ _index 1))
              (`self.Check Sides` _array_element _index _index_2)
              (`|ExecutionSequence` :!label _label_2
                (:`then_0`
                  (break))
                (:`then_1`
                  (goto _label :!via `Break`))))
            (elif (or (== _index 3) (== _index 5))
              (`self.Check Sides` _array_element _index 3)
              (goto _label_2)
              (elif (or (== _index 7) (== _index 1))
                (`self.Check Sides` _array_element _index 1)
                (goto _label_2))))
          (else
            (goto _label_3 :!via `Close`))))
      (if (not (`self.Game end ?`))
        (`/Engine/EditorBlueprintResources/StandardMacros.Gate` true :!label _label_3
          (:`Exit`
            (set `self.Game end ?` true)))))
    (:`then_1`
      (goto _label_3 :!via `Open`))))

(fn `UserConstructionScript`
  (bind (_returnvalue_x _returnvalue_y _returnvalue_z) (`KismetMathLibrary.BreakVector` (`self.K2_GetActorLocation`)))
  (bind _cubes_spaces (`self.Cubes_Spaces`))
  (bind _column_size (`self.Column_size`))
  (bind _line_size (`self.Line_size`))
  (bind _grid_elements_count (`self.Grid_elements_count`))
  (for _index (range 1 (+ _column_size 1))
    (for _index_2 (range 1 (+ _line_size 1))
      (bind _returnvalue (`AddComponent|NODE_AddChildActorComponent-0` :`RelativeTransform` (`KismetMathLibrary.MakeTransform` (`KismetMathLibrary.MakeVector` (+ _returnvalue_x (* _cubes_spaces (- (`KismetMathLibrary.Conv_IntToDouble` _index_2) (/ (`KismetMathLibrary.Conv_IntToDouble` _line_size) 2.0)))) (+ _returnvalue_y (* _cubes_spaces (- (`KismetMathLibrary.Conv_IntToDouble` _index) (/ (`KismetMathLibrary.Conv_IntToDouble` _column_size) 2.0)))) _returnvalue_z))))
      (bind _asbox_bp (cast `/Game/Blueprints/Box_BP` (`ChildActorComponent.ChildActor` _returnvalue)))
      (set `/Game/Blueprints/Box_BP.Grid_ref` self _asbox_bp)
      (set `/Game/Blueprints/Box_BP.Index` _grid_elements_count _asbox_bp)
      (`/Game/Blueprints/Box_BP.Init index` _asbox_bp)
      (`/Engine/EditorBlueprintResources/StandardMacros.IncrementInt` _grid_elements_count
        (:`  `
          (`KismetArrayLibrary.Array_Add` (`self.Boxs`) _asbox_bp))))))