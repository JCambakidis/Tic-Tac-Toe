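; Box_BP is one clickable cell in a two-player circle-and-cross grid game, apparently tic-tac-toe.
; A first click while the game is live records the current player, shows that player's mesh, flips the grid's turn and calls its CheckEnd.
; The click also spawns a Niagara spark effect and plays a timeline that moves the box vertically from its stored start height.
; Initindex displays the cell's index as text.
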(event `self.ReceiveBeginPlay`
  (set `self.Init_Location` (`SceneComponent.K2_GetComponentLocation` (`self.Scene`))))

(event `self.ReceiveTick`
  (params (DeltaSeconds :type "Float (single-precision)")))

(event `self.Cube.OnClicked`
  (params (TouchedComponent :type "PrimitiveComponent Object Reference") (ButtonPressed :type "Key Structure"))
  (bind (_init_location_x _init_location_y _init_location_z) (`KismetMathLibrary.BreakVector` (`self.Init_Location`)))
  (bind (_init_location_x_2 _init_location_y_2 _init_location_z_2) (`KismetMathLibrary.BreakVector` (`self.Init_Location`)))
  (bind _grid_ref (`self.Grid_ref`))
  (bind _select_feedback (`self.Select_feedback`))
  (bind (_returnvalue_x _returnvalue_y) (`KismetMathLibrary.BreakVector` (`SceneComponent.K2_GetComponentLocation` (`self.Scene`))))
  (bind _player_turn (`/Game/Blueprints/Grid_BP.Player turn` _grid_ref))
  (if (and (not (`self.Clicked`)) (not (`/Game/Blueprints/Grid_BP.Game end ?` (`self.Grid_ref`))))
    (`|ExecutionSequence`
      (:`then_0`
        (set `self.Clicked` true)
        (switch `int` _player_turn
          (:`0`
            (set `self.Clicked_Player` _player_turn)
            (`StaticMeshComponent.SetStaticMesh` _select_feedback "/Game/Mesh/Circle_StaticMesh.Circle_StaticMesh")
            (set `/Game/Blueprints/Grid_BP.Player turn` 1 _grid_ref))
          (:`1`
            (set `self.Clicked_Player` _player_turn)
            (`StaticMeshComponent.SetStaticMesh` _select_feedback "/Game/Mesh/Cross_StaticMesh.Cross_StaticMesh")
            (set `/Game/Blueprints/Grid_BP.Player turn` 0 _grid_ref)))
        (`/Game/Blueprints/Grid_BP.Check End` _grid_ref))
      (:`then_1`
        (`NiagaraFunctionLibrary.SpawnSystemAtLocation` "/Game/Niagara/NS_Sparks_26.NS_Sparks_26" (`KismetMathLibrary.MakeVector` _init_location_x_2 _init_location_y_2 (+ _init_location_z_2 50.0)))
        (bind (_direction _z) (`Timeline|Click_mouvement` :!via `PlayFromStart`)
          (:`Update`
            (`SceneComponent.K2_SetWorldLocation` (`self.Scene`) (`KismetMathLibrary.MakeVector` _returnvalue_x _returnvalue_y (- _init_location_z _z)) false false)))))))

(event `Init index`
  (`TextRenderComponent.K2_SetText` (`self.TextRender`) (`KismetTextLibrary.Conv_IntToText` (`self.Index`) false false)))

(fn `UserConstructionScript`)